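; Parkour component for a Character that climbs, mantles or vaults obstacles in front of it when Do_Parkour fires.
; Sphere traces find the obstacle's facing, top and far side, then height and depth pick the action and montage.
; Start and End Motion Warping targets align the montage, with motion warping added at BeginPlay.
; The capsule drops collision and flies during playback, restoring walking on blend out or interruption.
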(event `self.ReceiveBeginPlay`
  (bind _ascharacter (cast `Character` (`self.GetOwner`)))
  (set `self.As Character` _ascharacter)
  (bind _returnvalue (`|AddComponentByClass` (`self.As Character`) "/Script/MotionWarping.MotionWarpingComponent"))
  (set `self.MotionWarping` _returnvalue))

(event `Do_Parkour`
  (if (not (`AnimInstance.IsAnyMontagePlaying` (`SkeletalMeshComponent.GetAnimInstance` (`Character.Mesh` (`self.As Character`)))))
    (`self.Obstacle Detection`)
    (if (`self.ObstacleDetected`)
      (`self.Obstacle Query`)
      (`self.Obstacle Action`)
      (if (not (`|EnumEquality` (`self.ParkourAction`) "NewEnumerator0"))
        (`self.SettingCharacter` "NoCollision" "MOVE_Flying")
        (`self.SetMotionWarpingTargets`)
        (`|PlayMontage` (`Character.Mesh` (`self.As Character`)) (`self.Montage to Play`)
          (:`OnBlendOut`
            _)
          (:`OnInterrupted`
            _))
        (`self.SettingCharacter` "QueryAndPhysics" "MOVE_Walking")))))

(fn `Obstacle Action`
  (if (`self.IsParkourObstacleValid`)
    (bind _height (`self.Obstacle Height`))
    (if (> _height 120.0)
      (set `self.ParkourAction` "NewEnumerator1")
      (set `self.Montage to Play` "/Game/Parkour/Animation/Montages/Climb_Montage.Climb_Montage")
      (elif (`self.IsObstacleDeep`)
        (set `self.ParkourAction` "NewEnumerator2")
        (set `self.Montage to Play` "/Game/Parkour/Animation/Montages/Mantle_Montage.Mantle_Montage")
        (else
          (set `self.ParkourAction` "NewEnumerator3")
          (set `self.Montage to Play` "/Game/Parkour/Animation/Montages/Vault_Montage.Vault_Montage"))))
    (else
      (set `self.ParkourAction` "NewEnumerator0")
      (set `self.Montage to Play` null))))

(fn `Obstacle Detection`
  (bind _as_character (`self.As Character`))
  (bind _returnvalue (`Actor.K2_GetActorLocation` _as_character))
  (bind _outhit (`KismetSystemLibrary.SphereTraceSingleForObjects` _returnvalue (+ _returnvalue (* (`KismetMathLibrary.GetForwardVector` (`Actor.K2_GetActorRotation` _as_character)) 80.0)) 20.0 (`|MakeArray` "ObjectTypeQuery7" :!type "EObjectTypeQuery Enum")))
  (bind (_bblockinghit _binitialoverlap _time _distance _location _impactpoint _normal _impactnormal) (`GameplayStatics.BreakHitResult` _outhit))
  (set `self.ObstacleDetected` _bblockinghit)
  (if (`self.ObstacleDetected`)
    (set `self.ObjectDetectedLocation` _impactpoint)
    (bind (_returnvalue_roll _returnvalue_pitch _returnvalue_yaw) (`KismetMathLibrary.BreakRotator` (`KismetMathLibrary.NormalizedDeltaRotator` (`KismetMathLibrary.MakeRotFromX` _impactnormal) (struct :`Yaw` 180.0))))
    (set `self.ObstacleRotation` (`KismetMathLibrary.MakeRotator` 0.0 0.0 _returnvalue_yaw))))

(fn `Obstacle Height`
  (returns (Height :type "Float (double-precision)"))
  (bind (_returnvalue_x _returnvalue_y _returnvalue_z) (`KismetMathLibrary.BreakVector` (- (`self.ObstacleStartLocation`) (`SceneComponent.GetSocketLocation` (`Character.Mesh` (`self.As Character`)) "root"))))
  (return _returnvalue_z))

(fn `Obstacle Query`
  (bind _objectdetectedlocation (`self.ObjectDetectedLocation`))
  (bind _returnvalue (+ (`self.ObstacleStartLocation`) (* (`KismetMathLibrary.GetForwardVector` (`self.ObstacleRotation`)) 65.0)))
  (bind _outhit (`KismetSystemLibrary.SphereTraceSingle` (+ _objectdetectedlocation (0.0 0.0 200.0)) (- _objectdetectedlocation (0.0 0.0 10.0)) 0.0 "TraceTypeQuery1"))
  (bind (_bblockinghit _binitialoverlap _time _distance _location _impactpoint) (`GameplayStatics.BreakHitResult` _outhit))
  (set `self.IsParkourObstacleValid` (and _bblockinghit (not _binitialoverlap)))
  (set `self.ObstacleStartLocation` _impactpoint)
  (bind _outhit_2 (`KismetSystemLibrary.SphereTraceSingle` _returnvalue (- _returnvalue (0.0 0.0 250.0)) 15.0 "TraceTypeQuery1"))
  (bind (_bblockinghit_2 _binitialoverlap_2 _time_2 _distance_2 _location_2 _impactpoint_2 _normal _impactnormal _physmat _hitactor _hitcomponent _hitbonename _bonename _hititem _elementindex _faceindex _tracestart _traceend) (`GameplayStatics.BreakHitResult` _outhit_2))
  (set `self.IsObstacleDeep` _binitialoverlap_2)
  (set `self.ObstacleEndLocation` (`KismetMathLibrary.SelectVector` _impactpoint_2 _traceend _bblockinghit_2)))

(fn `SetMotionWarpingTargets`
  (switch `/Game/Parkour/E_Parkour` (`self.ParkourAction`)
    (:`NewEnumerator1`
      (bind _location_out (`self.WarpOffset` (`self.ObstacleStartLocation`) -45.0 -160.0))
      (`MotionWarpingComponent.AddOrUpdateWarpTargetFromLocationAndRotation` (`self.MotionWarping`) "Start" _location_out (`self.ObstacleRotation`))
      (bind _location_out_2 (`self.WarpOffset` (`self.ObstacleStartLocation`) 35.0 5.0))
      (`MotionWarpingComponent.AddOrUpdateWarpTargetFromLocationAndRotation` (`self.MotionWarping`) "End" _location_out_2 (`self.ObstacleRotation`)))
    (:`NewEnumerator2`
      (bind _location_out_3 (`self.WarpOffset` (`self.ObstacleStartLocation`)))
      (`MotionWarpingComponent.AddOrUpdateWarpTargetFromLocationAndRotation` (`self.MotionWarping`) "Start" _location_out_3 (`self.ObstacleRotation`))
      (bind _location_out_4 (`self.WarpOffset` (`self.ObstacleEndLocation`) 20.0 3.0))
      (`MotionWarpingComponent.AddOrUpdateWarpTargetFromLocationAndRotation` (`self.MotionWarping`) "End" _location_out_4 (`self.ObstacleRotation`)))
    (:`NewEnumerator3`
      (bind _location_out_5 (`self.WarpOffset` (`self.ObstacleStartLocation`) -15.0))
      (`MotionWarpingComponent.AddOrUpdateWarpTargetFromLocationAndRotation` (`self.MotionWarping`) "Start" _location_out_5 (`self.ObstacleRotation`))
      (bind _location_out_6 (`self.WarpOffset` (`self.ObstacleEndLocation`) 25.0 5.0))
      (`MotionWarpingComponent.AddOrUpdateWarpTargetFromLocationAndRotation` (`self.MotionWarping`) "End" _location_out_6 (`self.ObstacleRotation`)))))

(fn `SettingCharacter`
  (params (NewCollision :type "ECollisionEnabled Enum" :default "NoCollision") (NewMovementMode :type "EMovementMode Enum" :default "MOVE_None"))
  (bind _as_character (`self.As Character`))
  (`PrimitiveComponent.SetCollisionEnabled` (`Character.CapsuleComponent` _as_character) NewCollision)
  (`CharacterMovementComponent.SetMovementMode` (`Character.CharacterMovement` _as_character) NewMovementMode 0))

(fn `WarpOffset`
  (params (`Location In` :type "Vector Structure") (ForwardOffset :type "Float (double-precision)") (`Up Offset` :type "Float (double-precision)"))
  (returns (`Location Out` :type "Vector Structure"))
  (return (+ (+ `Location In` (`KismetMathLibrary.MakeVector` 0.0 0.0 `Up Offset`)) (* ForwardOffset (`KismetMathLibrary.GetForwardVector` (`self.ObstacleRotation`))))))